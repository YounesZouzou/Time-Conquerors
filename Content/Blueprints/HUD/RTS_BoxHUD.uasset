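; RTS HUD that handles drag-box selection of units and the middle panel that shows them.
; While dragging, DrawHUD draws the rectangle, selects units inside it, deselects those that leave, and clears any selected building.
; On release it builds a new middle panel, filling a grid with each selected unit's widget, or disposes of it when nothing is selected.
; Other events expose single selection, clearing and panel access.
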(event EventClearSelectedUnits
  (bind _selectedunits (Variables|Default|GetSelectedUnits))
  (for _array_element _selectedunits
    (Class|BISelectableInterface|DeselectThis(Message) _array_element))
  (Utilities|Array|Clear _selectedunits))

(event EventSelectSingleUnit
  (params (Unit :type Actor%20Object%20Reference))
  (Class|BISelectableInterface|SelectThis(Message) Unit)
  (Utilities|Array|AddUnique (Variables|Default|GetSelectedUnits) Unit))

(event EventBoxReleased
  ;[1 1 1] Box released
  (Variables|Default|SetisDrawing? false)
  (Variables|Default|SetRow 0)
  (Variables|Default|SetColumn 0)
  (bind _middlepanelwidget (CallFunction|CreateNewMiddlePanel))
  (Variables|Default|SetMiddlePanelWidget _middlepanelwidget)
  (if (Utilities|Array|IsEmpty (Variables|Default|GetSelectedUnits))
    (Class|BISelectableInterface|DisposeOfMiddlePanel(Message) (Variables|Default|GetMiddlePanelWidget))
    (else
      (bind _returnvalue (UserInterface|CreateWidget "/Game/UI/MiddlePanel/WB_Unit_Information_Menu.WB_Unit_Information_Menu_C"))
      (Class|CanvasPanel|AddChildtoCanvas (Variables|/Game/UI/WB_Middle_Panel.WB_Middle_Panel_C|GetCanvasPanel (Variables|Default|GetMiddlePanelWidget)) _returnvalue)
      ;[1 1 1] Needs improving
      (for _array_element (Variables|Default|GetSelectedUnits)
        (bind _asbp_parent_unit_class (Utilities|Casting|CastToBP_Parent_Unit_Class _array_element))
        (Utilities|PopulateUnitWidget (Variables|/Game/UI/MiddlePanel/WB_Unit_Information_Menu.WB_Unit_Information_Menu_C|GetUniformGridPanel _returnvalue) _asbp_parent_unit_class)
        (Utilities|AdjusttoPanel
          (:out
            (UserInterface|Viewport|AddtoViewport (Variables|Default|GetMiddlePanelWidget) 0)))))))

(event EventBoxPressed
  (bind _returnvalue (Game|GetPlayerController 0))
  (bind _middlepanelwidget (Variables|Default|GetMiddlePanelWidget))
  (bind (_locationx _locationy) (Game|Player|GetMousePosition _returnvalue))
  ;[1 1 1] Box Start
  (Variables|Default|SetisDrawing? true)
  (bind _output_get (Variables|Default|SetStartMousePosition (Math|Vector2D|MakeVector2D _locationx _locationy)))
  (Variables|Default|SetCurrentMousePosition _output_get)
  (if (Utilities|IsValid _middlepanelwidget)
    (Widget|RemovefromParent _middlepanelwidget)))

(event EventBoxHeld
  (bind _returnvalue (Game|GetPlayerController 0))
  (bind (_locationx _locationy) (Game|Player|GetMousePosition _returnvalue))
  ;[1 1 1] Box held
  (Variables|Default|SetCurrentMousePosition (Math|Vector2D|MakeVector2D _locationx _locationy)))

(event EventDisposeOfMiddlePanel
  (Widget|RemovefromParent (Variables|Default|GetMiddlePanelWidget)))

(event EventSetMiddlePanel
  (params (MiddlePanelWidget :type WB%20Middle%20Panel%20Object%20Reference))
  (Variables|Default|SetMiddlePanelWidget MiddlePanelWidget))

(event EventConfigureMiddlePanel
  (params (MiddlePanelWidget :type WB%20Middle%20Panel%20Object%20Reference))
  (bind _canvaspanel (Variables|/Game/UI/WB_Middle_Panel.WB_Middle_Panel_C|GetCanvasPanel (Variables|Default|GetMiddlePanelWidget)))
  (bind _returnvalue (Class|PanelWidget|GetChildat _canvaspanel 2))
  (bind _returnvalue_2 (Class|WidgetLayoutLibrary|SlotasCanvasSlot _returnvalue))
  (Class|CanvasPanelSlot|SetAnchors _returnvalue_2 (Utilities|Struct|MakeAnchors "(X=0.000000,Y=0.000000)" "(X=1.000000,Y=1.000000)"))
  (Class|CanvasPanelSlot|SetOffsets _returnvalue_2))

(event EventDrawHUD
  (params (SizeX :type Integer) (SizeY :type Integer))
  (bind _startmouseposition (Variables|Default|GetStartMousePosition))
  (bind _currentmouseposition (Variables|Default|GetCurrentMousePosition))
  ;[1 1 1] This part draws the rectangle from the first mouse position to the point u release the mouse
  (if (Variables|Default|GetisDrawing?)
    (HUD|DrawRect "(R=0.000000,G=0.044499,B=1.000000,A=0.467000)" (.x _startmouseposition) (.y _startmouseposition) (- (.x _currentmouseposition) (.x _startmouseposition)) (- (.y _currentmouseposition) (.y _startmouseposition)))
    ;[1 1 1] Put all actors under the rectangle drawn in the actors in rectangle array
    (bind _output_get (Variables|Default|SetActorsInRectangle (Class|HUD|GetActorsinSelectionRectangle "/Game/Blueprints/Units/BP_Parent_Unit_Class.BP_Parent_Unit_Class_C" (Variables|Default|GetStartMousePosition) (Variables|Default|GetCurrentMousePosition) false false)))
    ;[1 1 1] This puts an enable select decal command on all units in the array and adds them to the selected units array
    (for _array_element _output_get
      (Class|BISelectableInterface|SelectThis(Message) _array_element)
      (Utilities|Array|AddUnique (Variables|Default|GetSelectedUnits) _array_element)
      (Class|BIBuildingInterface|ClearSelectedBuilding(Message) (Game|GetPlayerController 0)))
    ;[1 1 1] This deselects the units within the rectangle that were at some point in it when the player did it but ended up not selected
    (for _array_element_2 (Variables|Default|GetSelectedUnits)
      (if (== (Utilities|Array|FindItem (Variables|Default|GetActorsInRectangle) _array_element_2) -1)
        (Class|BISelectableInterface|DeselectThis(Message) _array_element_2)
        (Utilities|Array|RemoveItem (Variables|Default|GetSelectedUnits) _array_element_2)))))

(fn ConstructionScript)

(fn CreateNewMiddlePanel
  (bind _returnvalue (UserInterface|CreateWidget "/Game/UI/WB_Middle_Panel.WB_Middle_Panel_C"))
  (return _returnvalue))

(fn GetMiddlePanel
  (return (Variables|Default|GetMiddlePanelWidget)))

(fn GrabSelectedUnits
  (return (Variables|Default|GetSelectedUnits)))