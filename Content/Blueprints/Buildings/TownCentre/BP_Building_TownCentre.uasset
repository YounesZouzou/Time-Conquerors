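; Town Centre building, a child of a parent building Blueprint, that offers a recruitment option for BP_Unit_FirstUnit.
; On BeginPlay it creates a WB_Recruitment_Item widget and sets its spawn reference to an existing BP_Unit_FirstUnit actor found with GetActorOfClass.
; It adds the widget to ListOfWidgetsToAdd and sets BuildingReference to itself before calling the parent BeginPlay.
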(event EventBeginPlay
  (bind _returnvalue (UserInterface|CreateWidget "/Game/UI/MiddlePanel/WB_Recruitment_Item.WB_Recruitment_Item_C"))
  (bind _returnvalue_2 (Actor|GetActorOfClass "/Game/Blueprints/Units/BP_Unit_FirstUnit.BP_Unit_FirstUnit_C"))
  (Variables|/Game/UI/MiddlePanel/WB_Recruitment_Item.WB_Recruitment_Item_C|SetUnitToSpawnReference _returnvalue _returnvalue_2)
  (Utilities|Array|AddUnique (Variables|Default|GetListOfWidgetsToAdd) _returnvalue)
  (Variables|Default|SetBuildingReference self)
  (|CallParentFunction))

(event Collision|EventActorBeginOverlap
  (params (OtherActor :type Actor%20Object%20Reference))
  (|CallParentFunction OtherActor) ; This node is disabled and will not be called.\nDrag off pins to build functionality.
)

(event EventTick
  (params (DeltaSeconds :type Float%20%28single-precision%29))
  (|CallParentFunction DeltaSeconds) ; This node is disabled and will not be called.\nDrag off pins to build functionality.
)

(fn ConstructionScript
  (|CallParentFunction))