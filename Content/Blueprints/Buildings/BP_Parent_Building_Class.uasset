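; Parent class for team-owned buildings that can be selected and recruit units from a production queue.
; BeginPlay builds the middle-panel recruitment UI from DT_BuildingAndItsUnits, which selection shows alongside a decal.
; A looping timer advances production using each unit class's default build time, then spawns the unit within SpawnPoint's bounds and applies its team.
; The construction script sets the team material from DT_MaterialsByTeam and initialises the health bar.
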(event Custom|ProcessQueue
  (bind _buildingreference (Variables|Default|GetBuildingReference))
  (bind _spawnpoint (Variables|BP_Parent_Building_Class_C|GetSpawnPoint _buildingreference))
  (bind (_origin _boxextent) (Collision|GetComponentBounds _spawnpoint))
  (if (Variables|Default|GetisProducingUnits?)
    (bind _output_get (Variables|Default|SetProductionTimeSpent (+ (Variables|Default|GetProductionTimeSpent) (Variables|Default|GetTimeBeforeCheckingQueue))))
    (bind _output_get_2 (Variables|Default|SetProductionProgress (/ _output_get (Variables|Default|GetProductionTime))))
    (if (>= _output_get_2 1.0)
      (Class|PanelWidget|RemoveChildat (Variables|/Game/UI/Gameplay/MiddlePanel/WB_Building_Recruitment_Menu.WB_Building_Recruitment_Menu_C|GetUniformGridPanelQueue (Variables|Default|GetRecruitmentMenuWidget)))
      (bind _returnvalue (Game|SpawnActorfromClass (Variables|Default|GetUnitToBeCreated) (Math|Transform|MakeTransform (.location (Math|Transform|MakeTransform (Math|Random|RandomPointinBoundingBox _origin _boxextent))) "0, 0, 0" "1.000000,1.000000,1.000000") "AdjustIfPossibleButDontSpawnIfColliding" "MultiplyWithRoot" 0 0))
      (Variables|/Game/Blueprints/Units/BP_Parent_Unit_Class.BP_Parent_Unit_Class_C|SetTeamNumber _returnvalue (Variables|Default|GetTeamNumber))
      (Default|UpdateMaterialtoTeam _returnvalue)
      (Variables|Default|SetProductionProgress 0.0)
      (Variables|Default|SetProductionTimeSpent 0.0)
      (Variables|Default|SetUnitToBeCreated 0)
      (Variables|Default|SetisProducingUnits? false))
    (elif (> (Utilities|Array|Length (Variables|Default|GetProductionQueue)) 0)
      (bind _output_get_3 (Variables|Default|SetUnitToBeCreated (Utilities|Array|Get(acopy) (Variables|Default|GetProductionQueue))))
      (Variables|Default|SetProductionTime (.ProductionTime (Utilities|GetClassDefaults _output_get_3)))
      (Utilities|Array|RemoveIndex (Variables|Default|GetProductionQueue))
      (Variables|Default|SetisProducingUnits? true))))

(event EventBeginPlay
  (Utilities|FlowControl|Sequence
    (:then_0
      ;[1 1 1] Create middle panel widget
      (Utilities|CreateMiddlePanel
        (:out
          ;[1 1 1] Create the building widget then add it to the middle panel and finally adjust the anchors to fit the panel
          (CallFunction|CreateBuildingWidget)
          (Utilities|PopulateCentrewithWidgets
            (:NewParam2
              ;[1 1 1] Populate the building widget with its recruitable unit widgets
              (CallFunction|PopulateBuildingWidgetUnits))))))
    (:then_1
      (Utilities|Time|SetTimerbyEvent (delegate Custom|ProcessQueue) (Variables|Default|GetTimeBeforeCheckingQueue) true))))

(event EventAddWidgettoProductionQueue
  (params (UnitToAdd :type BP%20Parent%20Unit%20Class%20Class%20Reference))
  (bind _returnvalue (UserInterface|CreateWidget "/Game/UI/Gameplay/MiddlePanel/WB_Recruitment_Queue_Item.WB_Recruitment_Queue_Item_C"))
  (Variables|/Game/UI/Gameplay/MiddlePanel/WB_Recruitment_Queue_Item.WB_Recruitment_Queue_Item_C|SetBuildingReference _returnvalue self)
  (Variables|/Game/UI/Gameplay/MiddlePanel/WB_Recruitment_Queue_Item.WB_Recruitment_Queue_Item_C|SetUnitToSpawnReference _returnvalue UnitToAdd)
  (Utilities|Array|Add (Variables|Default|GetUnitInQueueWidgets) _returnvalue)
  (bind _returnvalue_2 (Class|UniformGridPanel|AddChildtoUniformGrid (Variables|/Game/UI/Gameplay/MiddlePanel/WB_Building_Recruitment_Menu.WB_Building_Recruitment_Menu_C|GetUniformGridPanelQueue (Variables|Default|GetRecruitmentMenuWidget)) _returnvalue 0 (Variables|Default|GetQueueColumn)))
  (Layout|GridSlot|SetVerticalAlignment _returnvalue_2 "VAlign_Fill")
  (Layout|GridSlot|SetHorizontalAlignment _returnvalue_2 "HAlign_Fill")
  (Variables|Default|SetQueueColumn (+ (Variables|Default|GetQueueColumn) 1)))

(event EventSelectThis
  (Rendering|SetVisibility (Variables|Default|GetSelectDecal) true false)
  (UserInterface|Viewport|AddtoViewport (Variables|Default|GetMiddlePanelWidget) 0))

(event EventAddUnittoProductionQueue
  (params (UnitToCreate :type BP%20Parent%20Unit%20Class%20Class%20Reference))
  (Utilities|Array|Add (Variables|Default|GetProductionQueue) UnitToCreate))

(event EventDeselectThis
  (Rendering|SetVisibility (Variables|Default|GetSelectDecal) false false)
  (Widget|RemovefromParent (Variables|Default|GetMiddlePanelWidget)))

(event EventRemoveWidgetfromProductionQueue
  (params (WidgetToRemove :type WB%20Recruitment%20Queue%20Item%20Object%20Reference))
  (Utilities|Array|RemoveItem (Variables|Default|GetUnitInQueueWidgets) WidgetToRemove)
  (Class|PanelWidget|RemoveChild (Variables|/Game/UI/Gameplay/MiddlePanel/WB_Building_Recruitment_Menu.WB_Building_Recruitment_Menu_C|GetUniformGridPanelQueue (Variables|Default|GetRecruitmentMenuWidget)) WidgetToRemove))

(event EventRemoveUnitfromProductionQueue
  (params (UnitToRemove :type BP%20Parent%20Unit%20Class%20Class%20Reference))
  (bind _productionqueue (Variables|Default|GetProductionQueue))
  (Utilities|Array|RemoveIndex _productionqueue (Utilities|Array|FindItem _productionqueue UnitToRemove)))

(fn ConstructionScript
  (bind _returnvalue (Utilities|GetDataTableRow "/Game/Data/MaterialData/DT_MaterialsByTeam.DT_MaterialsByTeam" (Utilities|String|StringToName (Utilities|String|ToString(Integer) (Variables|Default|GetTeamNumber))))
    (:then
      (Rendering|Material|SetMaterial (Variables|Default|GetBuildingMesh) 0 (.BuildingMaterial (Utilities|Struct|BreakS_MaterialsByTeam _returnvalue)))
      (bind _aswb_healthbar (Utilities|Casting|CastToWB_Healthbar (UserInterface|GetWidget (Variables|Default|GetHealthBarWidget))))
      (Variables|/Script/UMG.ProgressBar|SetPercent (Variables|/Game/UI/Gameplay/AboveUnits/WB_Healthbar.WB_Healthbar_C|GetHealthBar _aswb_healthbar) (Variables|Default|GetHealth)))))

(fn CreateBuildingWidget
  (bind _returnvalue (UserInterface|CreateWidget "/Game/UI/Gameplay/MiddlePanel/WB_Building_Recruitment_Menu.WB_Building_Recruitment_Menu_C"))
  (bind _output_get (Variables|Default|SetRecruitmentMenuWidget _returnvalue))
  (Variables|/Game/UI/Gameplay/MiddlePanel/WB_Building_Recruitment_Menu.WB_Building_Recruitment_Menu_C|SetBuildingReference _output_get (Variables|Default|GetBuildingReference))
  (Widget|Panel|AddChild (Variables|/Game/UI/Gameplay/WB_Middle_Panel.WB_Middle_Panel_C|GetCanvasPanel (Variables|Default|GetMiddlePanelWidget)) _output_get)
  (Class|BISelectableInterface|ConfigureMiddlePanel(Message) (HUD|GetHUD (Game|GetPlayerController 0))))

(fn PopulateBuildingWidgetUnits
  (Variables|Default|SetRecruitColumn 0)
  (for _array_element (Variables|Default|GetListOfWidgetsToAdd)
    (Variables|/Game/UI/Gameplay/MiddlePanel/WB_Recruitment_Item.WB_Recruitment_Item_C|SetBuildingReference _array_element self)
    (bind _returnvalue (Class|UniformGridPanel|AddChildtoUniformGrid (Variables|/Game/UI/Gameplay/MiddlePanel/WB_Building_Recruitment_Menu.WB_Building_Recruitment_Menu_C|GetUniformGridPanel (Variables|Default|GetRecruitmentMenuWidget)) _array_element 0 (Variables|Default|GetRecruitColumn)))
    (Layout|GridSlot|SetVerticalAlignment _returnvalue "VAlign_Fill")
    (Layout|GridSlot|SetHorizontalAlignment _returnvalue "HAlign_Fill")
    (Variables|Default|SetRecruitColumn (+ (Variables|Default|GetRecruitColumn) 1))))

(fn CreateNewMiddlePanel
  (return 0))

(fn GetMiddlePanel
  (return 0))

(fn GetTeam
  (return (Variables|Default|GetTeamNumber)))

(fn GrabSelectedUnits
  (return 0))