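; Parent Blueprint for resource actors, with four arrow-marked slots around a static mesh.
; The Construction Script caches the mesh location, collects the slot arrows, and maps each to its world location and a false state flag.
; BeginPlay spawns a persistent cursor effect at each SlotsVectorPositions entry, an array not filled in these graphs.
; GetResourceType exposes the resource type, while GetResources is an empty stub.
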(event EventBeginPlay
  (for _array_element (Variables|Default|GetSlotsVectorPositions)
    (Niagara|SpawnSystematLocation "/Game/Cursor/FX_Cursor.FX_Cursor" _array_element "0, 0, 0" "1.000000,1.000000,1.000000" false)))

(event EventTick
  (params (DeltaSeconds :type Float%20%28single-precision%29)))

(fn ConstructionScript
  (bind _slot1 (Variables|Default|GetSlot1))
  (bind _slot2 (Variables|Default|GetSlot2))
  (bind _slot3 (Variables|Default|GetSlot3))
  (bind _slot4 (Variables|Default|GetSlot4))
  (bind _arrows (Variables|Default|GetArrows))
  (Variables|Default|SetMeshLocation (Transformation|GetWorldLocation (Variables|Default|GetStaticMesh)))
  (Utilities|FlowControl|Sequence
    (:then_0
      (Utilities|FlowControl|Sequence
        (:then_0
          (Utilities|Map|Add (Variables|Default|GetArrowAndLocation) _slot1 (Transformation|GetWorldLocation _slot1)))
        (:then_1
          (Utilities|Map|Add (Variables|Default|GetArrowAndLocation) _slot2 (Transformation|GetWorldLocation _slot2)))
        (:then_2
          (Utilities|Map|Add (Variables|Default|GetArrowAndLocation) _slot3 (Transformation|GetWorldLocation _slot3)))
        (:then_3
          (Utilities|Map|Add (Variables|Default|GetArrowAndLocation) _slot4 (Transformation|GetWorldLocation _slot4)))))
    (:then_1
      (Utilities|FlowControl|Sequence
        (:then_0
          (Utilities|Array|Add _arrows (Variables|Default|GetSlot1)))
        (:then_1
          (Utilities|Array|Add _arrows (Variables|Default|GetSlot2)))
        (:then_2
          (Utilities|Array|Add _arrows (Variables|Default|GetSlot3)))
        (:then_3
          (Utilities|Array|Add _arrows (Variables|Default|GetSlot4)))))
    (:then_2
      (for _array_element (Variables|Default|GetArrows)
        (Utilities|Map|Add (Variables|Default|GetArrowAndState) _array_element false)))))

(fn GetResources
  (return "NewEnumerator0"))

(fn GetResourceType
  (return (Variables|Default|GetResourceType)))