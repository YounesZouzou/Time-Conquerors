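; Base Character class for selectable, commandable units, with team identity and health display.
; Selection toggles a decal and health bar and creates or removes a selected-unit UI item linked to the unit; move commands restart AI MoveTo.
; Construction applies walk speed and initial health, while a separate function sets team material from a data table.
; Health-bar camera-facing logic is disconnected, and the panel and selection-grab functions are empty stubs.
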(event EventBeginPlay)

(event Collision|EventActorBeginOverlap
  (params (OtherActor :type Actor%20Object%20Reference)))

(event EventTick
  (params (DeltaSeconds :type Float%20%28single-precision%29)))

(event EventUnitMoveCommand
  (params (Location :type Vector :default "0, 0, 0"))
  (bind _self self)
  (bind _returnvalue (AI|GetAIController _self))
  (AI|Navigation|StopMovement _returnvalue)
  (AI|AIMoveTo _returnvalue Location 0 1e+01 "Default" "Default" true true))

(event EventSelectThis
  (Rendering|SetVisibility (Variables|Default|GetSelectDecal) true false)
  (Rendering|SetVisibility (Variables|Default|GetHealthBarWidget) true false)
  (bind _returnvalue (UserInterface|CreateWidget "/Game/UI/MiddlePanel/WB_SelectedUnit_Item.WB_SelectedUnit_Item_C"))
  (bind _output_get (Variables|Default|SetSelectedUnitWidget _returnvalue))
  (Variables|/Game/UI/MiddlePanel/WB_SelectedUnit_Item.WB_SelectedUnit_Item_C|SetUnitReference _output_get self))

(event EventDeselectThis
  (Rendering|SetVisibility (Variables|Default|GetSelectDecal) false false)
  (Rendering|SetVisibility (Variables|Default|GetHealthBarWidget) false false)
  (Widget|RemovefromParent (stale EventSelectThis _returnvalue)))

(fn ConstructionScript
  (Variables|/Script/Engine.CharacterMovementComponent|SetMaxWalkSpeed (Variables|Character|GetCharacterMovement) (Variables|Default|GetMaxWalkSpeed))
  (bind _aswb_healthbar (Utilities|Casting|CastToWB_Healthbar (UserInterface|GetWidget (Variables|Default|GetHealthBarWidget))))
  (Variables|/Script/UMG.ProgressBar|SetPercent (Variables|/Game/UI/WB_Healthbar.WB_Healthbar_C|GetHealthBar _aswb_healthbar) (Variables|Default|GetHealth)))

(fn UpdateMaterialtoTeam
  (bind _returnvalue (Utilities|GetDataTableRow "/Game/Data/MaterialData/DT_MaterialsByTeam.DT_MaterialsByTeam" (Utilities|String|StringToName (Utilities|String|ToString(Integer) (Variables|Default|GetTeamNumber))))
    (:then
      (Rendering|Material|SetMaterial (Variables|Character|GetMesh) 0 (.UnitMaterial (Utilities|Struct|BreakS_MaterialsByTeam _returnvalue))))))

(fn CreateNewMiddlePanel
  (return 0))

(fn GetMiddlePanel
  (return 0))

(fn GetTeam
  (return (Variables|Default|GetTeamNumber)))

(fn GrabSelectedUnits
  (return 0))