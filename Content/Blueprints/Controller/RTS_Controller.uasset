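; RTS player controller handling box selection, building placement, unit orders and resource spending.
; A ghost building follows cursor traces on Tick, tinted green or red by hit actor and team town-centre distance, then spawns on left click.
; Right click cancels placement and sends selected units to move or workers to resources via interface messages.
; BeginPlay creates the main HUD widget, whose top panel tracks resources, and fills its building menu from a DataTable.
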(event EventTick
  (params (DeltaSeconds :type Float%20%28single-precision%29))
  (bind (_hitresult _returnvalue) (Game|Player|GetHitResultUnderCursorbyChannel "TraceTypeQuery2" true))
  (bind (_bblockinghit _binitialoverlap _time _distance _location _impactpoint _normal _impactnormal _physmat _hitactor) (Collision|BreakHitResult _hitresult))
  (if (Variables|Default|GetisBuildingModeEnabled?)
    (if _returnvalue
      (if (Utilities|BuildingDontBuildonLimit _hitactor)
        (Default|SetMaterialRed (Variables|Default|GetBuildingActor) :!label _label)
        (Transformation|SetWorldLocation (Variables|/Game/Blueprints/Buildings/BP_Parent_Building_Class.BP_Parent_Building_Class_C|GetBuildingMesh (Variables|Default|GetBuildingActor)) _location false false)
        (Variables|Default|SetcanPlaceBuilding? false)
        (else
          (Utilities|LookforClosestTownCentre _location
            (:out
              (if (>= (Variables|Default|GetClosestTownCentreDistance) (Variables|Default|GetTownCentreBuildingDistance))
                (goto _label)
                (else
                  (Transformation|SetWorldLocation (Variables|/Game/Blueprints/Buildings/BP_Parent_Building_Class.BP_Parent_Building_Class_C|GetBuildingMesh (Variables|Default|GetBuildingActor)) _location false false)
                  (Default|SetMaterialGreen (Variables|Default|GetBuildingActor))
                  (Variables|Default|SetcanPlaceBuilding? true))))))))
    (elif (Variables|Default|GetleftMousePressed?)
      (Class|BIBoxInterface|BoxHeld(Message) (HUD|GetHUD)))))

(event EventBeginPlay
  ;[0.05098 0.05098 0.05098] Add Mapping Context
  (Utilities|IsValid (PlayerController|LocalPlayerSubsystems|GetEnhancedInputLocalPlayerSubsystem)
    (:Is%20Valid
      (Input|SetInputModeGameandUI self 0 "LockAlways" false false)
      (Utilities|FlowControl|Sequence
        (:then_0
          (bind _returnvalue (UserInterface|CreateWidget "/Game/UI/Menu/Settings/WB_Settings_Menu.WB_Settings_Menu_C"))
          (Default|Setall _returnvalue))
        (:then_1
          ;[1 1 1] Add main panel
          (bind _returnvalue_2 (UserInterface|CreateWidget "/Game/UI/Gameplay/WB_Main_Window.WB_Main_Window_C"))
          (Variables|Default|SetMainWindowPanel _returnvalue_2)
          (UserInterface|Viewport|AddtoViewport (Variables|Default|GetMainWindowPanel) 0)
          (Variables|Default|SetbShowMouseCursor true)
          ;[1 1 1] Add buildings to building menu
          (Utilities|PopulateBuildingMenu))
        (:then_2
          ;[1 0 0.02862] DEBUG
          (Development|ExecuteConsoleCommand "RebuildNavigation" 0))))))

(event EventPurchaseUnit
  (params (UnitPurchased :type BP%20Parent%20Unit%20Class%20Class%20Reference))
  (bind _unitcost (Utilities|GetClassDefaults UnitPurchased))
  (bind _keys (Utilities|Map|Keys _unitcost))
  (for _array_element _keys
    (CallFunction|DecreaseResourceAmount _array_element (.Value (Utilities|Map|Find _unitcost _array_element)))))

(event EventDecreaseResourceAmount
  (params (TypeToDecrease :type E_ResourceTypes%20Enum :default "NewEnumerator0") (Amount :type Integer))
  (Class|BIResourceInterface|DecreaseResourceAmount(Message) (Variables|/Game/UI/Gameplay/WB_Main_Window.WB_Main_Window_C|GetWB_Top_Panel (Variables|Default|GetMainWindowPanel)) TypeToDecrease Amount))

(event EventClearSelectedBuilding
  (Utilities|IsValid (Variables|Default|GetSelectedBuilding)
    (:Is%20Valid
      (Class|BISelectableInterface|DeselectThis(Message) (Variables|Default|GetSelectedBuilding))
      (Variables|Default|SetSelectedBuilding 0))))

(event EventCreateUnit
  (params (Building :type BP%20Parent%20Building%20Class%20Object%20Reference) (UnitToCreate :type BP%20Parent%20Unit%20Class%20Class%20Reference))
  (bind _currentresources (Class|BIResourceInterface|GetResources(Message) (Variables|/Game/UI/Gameplay/WB_Main_Window.WB_Main_Window_C|GetWB_Top_Panel (Variables|Default|GetMainWindowPanel))))
  (bind _canpurchaseunit_ (Class|BIRecruitingInterface|CanPurchaseUnit?(Message) self UnitToCreate _currentresources))
  (if _canpurchaseunit_
    (Class|BIRecruitingInterface|AddWidgettoProductionQueue(Message) Building UnitToCreate)
    (Class|BIRecruitingInterface|AddUnittoProductionQueue(Message) Building UnitToCreate)
    (CallFunction|PurchaseUnit UnitToCreate)
    (else
      (Development|PrintString "Can not afford unit "))))

(event EventEnableBuildingMode
  (Variables|Default|SetisBuildingModeEnabled? true))

(event EventDisableBuildingMode
  (Variables|Default|SetisBuildingModeEnabled? false))

(event EventPurchaseBuilding
  (params (BuildingPurchased :type BP%20Parent%20Building%20Class%20Class%20Reference))
  (bind _buildingcost (Utilities|GetClassDefaults BuildingPurchased))
  (bind _keys (Utilities|Map|Keys _buildingcost))
  (for _array_element _keys
    (CallFunction|DecreaseResourceAmount _array_element (.Value (Utilities|Map|Find _buildingcost _array_element)))))

(event EventGetBuildingtobePlaced
  (params (Building :type BP%20Parent%20Building%20Class%20Class%20Reference))
  (Utilities|IsValid (Variables|Default|GetBuildingActor)
    (:Is%20Valid
      (Actor|DestroyActor (Variables|Default|GetBuildingActor)))
    (:Is%20Not%20Valid
      _))
  (bind _output_get (Variables|Default|SetBuildingToBePlaced Building))
  (bind _returnvalue (Game|SpawnActorfromClass _output_get (Math|Transform|MakeTransform "0, 0, 0" "0, 0, 0" "1.000000,1.000000,1.000000") "Undefined" "MultiplyWithRoot" 0 0))
  (bind _output_get_2 (Variables|Default|SetBuildingActor _returnvalue))
  (Default|SetMaterialGreen _output_get_2)
  (Collision|SetCollisionEnabled (Variables|/Game/Blueprints/Buildings/BP_Parent_Building_Class.BP_Parent_Building_Class_C|GetBuildingMesh _output_get_2) "NoCollision"))

(event EventIncreaseResourceAmount
  (params (TypeToIncrease :type E_ResourceTypes%20Enum :default "NewEnumerator0") (Amount :type Integer))
  (Class|BIResourceInterface|IncreaseResourceAmount(Message) (Variables|/Game/UI/Gameplay/WB_Main_Window.WB_Main_Window_C|GetWB_Top_Panel (Variables|Default|GetMainWindowPanel)) TypeToIncrease Amount))

(event EventRefundUnit
  (params (UnitPurchased :type BP%20Parent%20Unit%20Class%20Class%20Reference))
  (bind _unitcost (Utilities|GetClassDefaults UnitPurchased))
  (bind _keys (Utilities|Map|Keys _unitcost))
  (for _array_element _keys
    (CallFunction|IncreaseResourceAmount _array_element (.Value (Utilities|Map|Find _unitcost _array_element)))))

(event Input|MouseEvents|LeftMouseButton
  (params (Key :type Key%20Structure))
  (bind _returnvalue (HUD|GetHUD))
  (:Pressed
    ;[1 1 1] Spawning building on the left click location based on what widget was clicked
    (bind _output_get (Variables|Default|SetLeftClickLocation (.Location (Collision|BreakHitResult (.HitResult (Game|Player|GetHitResultUnderCursorbyChannel "TraceTypeQuery1" false))))))
    (if (and (Variables|Default|GetisBuildingModeEnabled?) (Variables|Default|GetcanPlaceBuilding?))
      (bind _returnvalue_2 (Game|SpawnActorfromClass (Variables|Default|GetBuildingToBePlaced) (Math|Transform|MakeTransform _output_get (Transformation|GetActorRotation (Variables|Default|GetBuildingActor)) "1.000000,1.000000,1.000000") "Undefined" "MultiplyWithRoot" 0 0))
      (Actor|DestroyActor (Variables|Default|GetBuildingActor))
      (Class|BIBuildingInterface|GenerateResourceBuilding(Message) _returnvalue_2)
      (CallFunction|PurchaseBuilding (Variables|Default|GetBuildingToBePlaced))
      (Variables|Default|SetisBuildingModeEnabled? false))
    (Variables|Default|SetleftMousePressed? true)
    (Utilities|HandleBuildingClick)
    (Class|BIBoxInterface|BoxPressed(Message) _returnvalue))
  (:Released
    (Variables|Default|SetleftMousePressed? false)
    (Class|BIBoxInterface|BoxReleased(Message) _returnvalue)))

(event Input|MouseEvents|RightMouseButton
  (params (Key :type Key%20Structure))
  (bind _hitresult (Game|Player|GetHitResultUnderCursorbyChannel "TraceTypeQuery1" true))
  (bind _buildingactor (Variables|Default|GetBuildingActor))
  (bind (_bblockinghit _binitialoverlap _time _distance _location _impactpoint _normal _impactnormal _physmat _hitactor) (Collision|BreakHitResult _hitresult))
  (:Pressed
    ;[1 1 1] When right clicking build mode is disabled
    (Variables|Default|SetisBuildingModeEnabled? false)
    (CallFunction|DisableBuildingMode)
    (Utilities|IsValid _buildingactor
      (:Is%20Valid
        (Actor|DestroyActor _buildingactor))
      (:Is%20Not%20Valid
        _))
    (Variables|Default|SetRightClickedActor _hitactor)
    (if (Utilities|ClassIsChildOf (Utilities|GetClass _hitactor) "/Game/Blueprints/Resources/BP_Parent_Resource_Class.BP_Parent_Resource_Class_C")
      (bind _units (Class|BISelectableInterface|GrabSelectedUnits(Message) (HUD|GetHUD)))
      (for _array_element _units
        (if (Utilities|DoesObjectImplementInterface _array_element "/Game/Blueprints/Interfaces/BI_Worker_Interface.BI_Worker_Interface_C")
          (Class|BIWorkerInterface|SetIsWorking(Message) _array_element (Variables|Default|GetRightClickedActor))))
      (else
        (Variables|Default|SetRightClickLocation _location)
        (bind _units_2 (Class|BISelectableInterface|GrabSelectedUnits(Message) (HUD|GetHUD)))
        (for _array_element_2 _units_2
          (if (== _array_element_2 "/Game/Blueprints/Units/Non-Combat/BP_Worker.BP_Worker")
            (Class|BIWorkerInterface|SetIsNotWorking(Message) _array_element_2))
          (bind _teamnumber (Class|BISelectableInterface|GetTeam(Message) (Variables|Default|GetRightClickedActor)))
          (if (== _teamnumber 0)
            (Utilities|IsValid _array_element_2
              (:Is%20Valid
                (Class|BICommandInterface|UnitMoveCommandVector(Message) _array_element_2 (Variables|Default|GetRightClickLocation))))))
        (Niagara|SpawnSystematLocation "/Game/Cursor/FX_Cursor.FX_Cursor" (Variables|Default|GetRightClickLocation))))))

(fn ConstructionScript)

(fn Moveto
  (params (Location :type Vector))
  (AI|Navigation|SimpleMovetoLocation self Location)
  (Niagara|SpawnSystematLocation (Variables|Input|GetFXCursor) Location))

(fn Follow
  (params (Location :type Vector))
  (bind _returnvalue (Pawn|GetControlledPawn))
  (Pawn|Input|AddMovementInput _returnvalue (Math|Vector|GetUnitDirection(Vector) (Transformation|GetActorLocation _returnvalue) Location) 1.0 false))

(fn GetLocationUnderCursor
  (bind _hitresult (Game|Player|GetHitResultUnderCursorbyChannel "TraceTypeQuery1" true))
  (bind (_bblockinghit _binitialoverlap _time _distance _location) (Collision|BreakHitResult _hitresult))
  (return _bblockinghit _location))

(fn GetLocationUnderFinger
  (bind _hitresult (Class|PlayerController|GetHitResultUnderFingerbyChannel "Touch1" "TraceTypeQuery1" false))
  (bind (_bblockinghit _binitialoverlap _time _distance _location) (Collision|BreakHitResult _hitresult))
  (return _bblockinghit _location))

(fn CanPurchaseUnit?
  (params (UnitToPurchase :type BP%20Parent%20Unit%20Class%20Class%20Reference) (CurrentResources :type Map%20of%20E_ResourceTypes%20Enums%20to%20Integers :default "NewEnumerator0"))
  (bind _unitcost (Utilities|GetClassDefaults UnitToPurchase))
  (bind _keys (Utilities|Map|Keys _unitcost))
  (bind _array_element (Utilities|Array|ForEachLoopwithBreak _keys)
    (:LoopBody
      (if (< (- (.Value (Utilities|Map|Find CurrentResources _array_element)) (.Value (Utilities|Map|Find _unitcost _array_element))) 0)
        (return false)))
    (:Completed
      (return true))))

(fn CreateNewMiddlePanel
  (return 0))

(fn GetBuildingActor
  (return (Variables|Default|GetBuildingActor)))

(fn GetIsAlive
  (return false))

(fn GetMiddlePanel
  (return 0))

(fn GetResources
  (return (Variables|Default|GetPlayerResources)))

(fn GetResourceType
  (return "NewEnumerator0"))

(fn GetTeam
  (return 0))

(fn GrabSelectedUnits
  (return 0))

(fn IsinBuildingMode?
  (return (Variables|Default|GetisBuildingModeEnabled?)))