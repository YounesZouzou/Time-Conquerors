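; Damage system Blueprint component that tracks Health, MaxHealth and an IsDead flag for its owner.
; Heal adds health clamped between zero and MaxHealth, while TakeDamage subtracts a DamageInfo amount without clamping and sets IsDead at zero or below.
; Both functions act only while alive, and non-lethal hits just print the DamageResponse enum to screen.
; Getters expose current and max health; the event graph is unused.
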(event EventBeginPlay)

(event EventTick
  (params (DeltaSeconds :type Float%20%28single-precision%29)))

(fn Heal
  (params (Amount :type Float%20%28double-precision%29))
  (if (not (Variables|Default|GetisDead?))
    (bind _output_get (Variables|Default|SetHealth (Math|Float|Clamp(Float) (+ Amount (Variables|Default|GetHealth)) 0.0 (Variables|Default|GetMaxHealth))))
    (return _output_get)))

(fn TakeDamage
  (params (DamageInfo :type S%20Damage%20Info%20Structure))
  (bind (_amount _damageresponse) (Utilities|Struct|BreakS_DamageInfo DamageInfo))
  (if (not (Variables|Default|GetisDead?))
    (bind _output_get (Variables|Default|SetHealth (- (Variables|Default|GetHealth) _amount)))
    (if (<= _output_get 0.0)
      (Variables|Default|SetisDead? true)
      (else
        (Development|PrintString (Utilities|String|EnumtoString _damageresponse))))
    (return true)))

(fn GetCurrentHealth
  (return (Variables|Default|GetHealth)))

(fn GetMaxHealth
  (return (Variables|Default|GetMaxHealth)))